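; VR player character that maps input to movement, camera turning and two-handed interaction, using floor-level tracking origin.
; Forward and right axes feed MoveForward and MoveRight, while the rotate axis triggers one RotateCamera step per near-full stick deflection, gated by HasTurned until release.
; Pick-up and fire actions forward press and release to LeftHand and RightHand, which handle pick up, drop, fire and end fire.
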(event EventBeginPlay
  (Class|HeadMountedDisplayFunctionLibrary|SetTrackingOrigin "Floor"))

(event Collision|EventActorBeginOverlap
  (params (OtherActor :type Actor%20Object%20Reference)))

(event EventTick
  (params (DeltaSeconds :type Float%20%28single-precision%29)))

(event Input|ActionEvents|InputActionLeftPickUp
  (params (Key :type Key%20Structure))
  (bind _lefthand (Variables|Default|GetLeftHand))
  (:Pressed
    (Class|VRMotionControllerComponent|PickUp _lefthand))
  (:Released
    (Class|VRMotionControllerComponent|Drop _lefthand)))

(event Input|ActionEvents|InputActionRightPickUp
  (params (Key :type Key%20Structure))
  (bind _righthand (Variables|Default|GetRightHand))
  (:Pressed
    (Class|VRMotionControllerComponent|PickUp _righthand))
  (:Released
    (Class|VRMotionControllerComponent|Drop _righthand)))

(event Input|ActionEvents|InputActionVRFireLeft
  (params (Key :type Key%20Structure))
  (:Pressed
    (Class|VRMotionControllerComponent|Fire (Variables|Default|GetLeftHand)))
  (:Released
    (Class|VRMotionControllerComponent|EndFire (Variables|Default|GetLeftHand))))

(event Input|ActionEvents|InputActionVRFireRight
  (params (Key :type Key%20Structure))
  (:Pressed
    (Class|VRMotionControllerComponent|Fire (Variables|Default|GetRightHand)))
  (:Released
    (Class|VRMotionControllerComponent|EndFire (Variables|Default|GetRightHand))))

(event Input|AxisEvents|InputAxisVRMoveForward
  (params (AxisValue :type Float%20%28single-precision%29))
  (Class|VRCharacter|MoveForward AxisValue))

(event Input|AxisEvents|InputAxisVRMoveRight
  (params (AxisValue :type Float%20%28single-precision%29))
  (Class|VRCharacter|MoveRight AxisValue))

(event Input|AxisEvents|InputAxisVRRotate
  (params (AxisValue :type Float%20%28single-precision%29))
  (if (or (> AxisValue 0.95) (< AxisValue -0.95))
    (if (not (Variables|Default|GetHasTurned))
      (if (> (Input|AxisValues|GetVRRotate) 0.0)
        (Class|VRCharacter|RotateCamera -1.0)
        (else
          (Class|VRCharacter|RotateCamera 1.0)))
      (Variables|Default|SetHasTurned true))
    (else
      (Variables|Default|SetHasTurned false))))

(fn ConstructionScript)