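; AI controller for spaceships that runs the spaceship behavior tree and feeds it radar targets.
; On begin play it sets up the blackboard and caches the pawn's RadarComponent.
; Each tick it sorts the radar's closest actor by its registrar target type into the aerial or ground blackboard key, clearing the other.
; With no contact, it clears all target keys and calls SetTargetActor on the spaceship pawn with no actor.
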(event EventBeginPlay
  (bind _returnvalue (Pawn|GetControlledPawn))
  (bind _returnvalue_2 (Actor|GetComponentbyClass _returnvalue "/Script/Spaceship.RadarComponent"))
  (CallFunction|SetupBehaviourTree)
  (Utilities|IsValid _returnvalue_2
    (:Is%20Valid
      (Variables|Default|SetRadarComponent _returnvalue_2))))

(event EventTick
  (params (DeltaSeconds :type Float%20%28single-precision%29))
  (CallFunction|SetBlackboardTargetValues))

(fn ConstructionScript)

(fn SetupBehaviourTree
  (bind _blackboardcomponent (Class|AIController|UseBlackboard "/Game/Behaviour/BB_SpaceshipData.BB_SpaceshipData"))
  (bind _output_get (Variables|Default|SetBlackboardComponent _blackboardcomponent))
  (bind _output_get_2 (LocalVariables|SetBB _output_get))
  (AI|Components|Blackboard|SetValueasBool _output_get_2 (LocalVariables|GetHasWaypoint) false)
  (AI|RunBehaviorTree "/Game/Behaviour/BehaviousTrees/BT_Spaceship.BT_Spaceship"))

(fn SetBlackboardTargetValues
  (bind _returnvalue (Class|RadarComponent|GetClosestActor (Variables|Default|GetRadarComponent)))
  (bind _output_get (LocalVariables|SetClosestActor _returnvalue))
  (Utilities|IsValid _output_get
    (:Is%20Valid
      (bind _output_get_2 (LocalVariables|SetRadarRegistrarComp (Actor|GetComponentbyClass (LocalVariables|GetClosestActor) "/Script/Spaceship.RadarRegistrarComponent")))
      (Utilities|IsValid _output_get_2
        (:Is%20Valid
          (bind _returnvalue_2 (Class|RadarRegistrarComponent|GetTargetType (LocalVariables|GetRadarRegistrarComp)))
          (switch Utilities|FlowControl|Switch|SwitchonETargetTypeEnum _returnvalue_2
            (:TT_Aerial
              (AI|Components|Blackboard|SetValueasObject (Variables|Default|GetBlackboardComponent) (Variables|Default|GetAerialActorKey) (LocalVariables|GetClosestActor))
              (AI|Components|Blackboard|ClearValue (Variables|Default|GetBlackboardComponent) (Variables|Default|GetGroundActorKey)))
            (:TT_Ground
              (AI|Components|Blackboard|SetValueasObject (Variables|Default|GetBlackboardComponent) (Variables|Default|GetGroundActorKey) (LocalVariables|GetClosestActor))
              (AI|Components|Blackboard|ClearValue (Variables|Default|GetBlackboardComponent) (Variables|Default|GetAerialActorKey)))))
        (:Is%20Not%20Valid
          (Development|PrintString "BP_SpaceshipAIController - SetBlackboardTargetValues - ERROR"))))
    (:Is%20Not%20Valid
      (AI|Components|Blackboard|ClearValue (Variables|Default|GetBlackboardComponent) (Variables|Default|GetTargetActorKey))
      (AI|Components|Blackboard|ClearValue (Variables|Default|GetBlackboardComponent) (Variables|Default|GetGroundActorKey))
      (AI|Components|Blackboard|ClearValue (Variables|Default|GetBlackboardComponent) (Variables|Default|GetAerialActorKey))
      (bind _asspaceship_pawn (Utilities|Casting|CastToSpaceshipPawn (Pawn|GetControlledPawn)))
      (Class|SpaceshipPawn|SetTargetActor _asspaceship_pawn))))