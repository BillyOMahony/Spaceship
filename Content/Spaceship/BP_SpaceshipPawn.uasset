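; Player spaceship pawn that passes flight input to a SpaceshipMovement component, which receives the Hull on BeginPlay.
; Throttle and directional thrust actions set pressed flags on that component, though ThrottleDown only ever sets true and ThrustUp only false.
; Each tick, the SpaceshipController's center-relative mouse position steers the camera, lerping Azimuth yaw from X and SpringArm pitch from Y between one shared pair of limits.
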(event EventBeginPlay
  (Class|SpaceshipMovementComponent|SetSpaceshipHull (Variables|Default|GetSpaceshipMovement) (Variables|Default|GetHull)))

(event Input|ActionEvents|InputActionThrottleUp
  (params (Key :type Key%20Structure))
  (bind _spaceshipmovement (Variables|Default|GetSpaceshipMovement))
  (:Pressed
    (Class|SpaceshipMovementComponent|SetThrottleUpPressed _spaceshipmovement true))
  (:Released
    (Class|SpaceshipMovementComponent|SetThrottleUpPressed _spaceshipmovement false)))

(event Input|ActionEvents|InputActionThrottleDown
  (params (Key :type Key%20Structure))
  (bind _spaceshipmovement (Variables|Default|GetSpaceshipMovement))
  (:Pressed
    (Class|SpaceshipMovementComponent|SetThrottleDownPressed _spaceshipmovement true))
  (:Released
    (Class|SpaceshipMovementComponent|SetThrottleDownPressed _spaceshipmovement true)))

(event Input|ActionEvents|InputActionThrustUp
  (params (Key :type Key%20Structure))
  (bind _spaceshipmovement (Variables|Default|GetSpaceshipMovement))
  (:Pressed
    (Class|SpaceshipMovementComponent|SetThrustUpPressed _spaceshipmovement false))
  (:Released
    (Class|SpaceshipMovementComponent|SetThrustUpPressed _spaceshipmovement false)))

(event Input|ActionEvents|InputActionThrustDown
  (params (Key :type Key%20Structure))
  (bind _spaceshipmovement (Variables|Default|GetSpaceshipMovement))
  (:Pressed
    (Class|SpaceshipMovementComponent|SetThrustDownPressed _spaceshipmovement true))
  (:Released
    (Class|SpaceshipMovementComponent|SetThrustDownPressed _spaceshipmovement false)))

(event Input|ActionEvents|InputActionThrustLeft
  (params (Key :type Key%20Structure))
  (bind _spaceshipmovement (Variables|Default|GetSpaceshipMovement))
  (:Pressed
    (Class|SpaceshipMovementComponent|SetThrustLeftPressed _spaceshipmovement true))
  (:Released
    (Class|SpaceshipMovementComponent|SetThrustLeftPressed _spaceshipmovement false)))

(event Input|ActionEvents|InputActionThrustRight
  (params (Key :type Key%20Structure))
  (bind _spaceshipmovement (Variables|Default|GetSpaceshipMovement))
  (:Pressed
    (Class|SpaceshipMovementComponent|SetThrustRightPressed _spaceshipmovement true))
  (:Released
    (Class|SpaceshipMovementComponent|SetThrustRightPressed _spaceshipmovement false)))

(event EventTick
  (params (DeltaSeconds :type Float%20%28single-precision%29))
  (Variables|Default|SetDeltaTime DeltaSeconds)
  (CallFunction|RotateCamera))

(fn ConstructionScript)

(fn SetAzimuthRotation
  (params (MouseX :type Float%20%28single-precision%29))
  (Transformation|SetRelativeRotation (Variables|Default|GetAzimuth) (Math|Rotator|MakeRotator 0.0 0.0 (Math|Float|Lerp (Variables|Default|GetCameraAzimultRotMax) (Variables|Default|GetCameraAzimuthRotMin) (/ (+ MouseX 1.0) 2.0))) false false))

(fn SetSpringArmRotation
  (params (MouseY :type Float%20%28single-precision%29))
  (Transformation|SetRelativeRotation (Variables|Default|GetSpringArm) (Math|Rotator|MakeRotator 0.0 (Math|Float|Lerp (Variables|Default|GetCameraAzimultRotMax) (Variables|Default|GetCameraAzimuthRotMin) (/ (+ MouseY 1.0) 2.0)) 0.0) false false))

(fn RotateCamera
  (bind _asspaceship_controller (Utilities|Casting|CastToSpaceshipController (Pawn|GetController)))
  (bind _returnvalue (Class|SpaceshipController|GetMousePositionRelativetoCenter _asspaceship_controller))
  (CallFunction|SetAzimuthRotation (.x _returnvalue))
  (CallFunction|SetSpringArmRotation (.y _returnvalue)))